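; controladorDeStamina is an actor Blueprint that prototypes a stamina counter, printed on screen as it changes.
; Tick feeds a two-second Delay, so ControleStamina drops by two periodically.
; Clicking the actor sets Confere2seg and adds one stamina.
; Tick clears Confere2seg just before testing it, so clicks never block the drain.
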(event `self.ReceiveTick`
  (params (DeltaSeconds :type "Float (single-precision)"))
  (`KismetSystemLibrary.Delay` 2.0)
  (set `self.confere2seg` false)
  (if (not (`self.confere2seg`))
    (bind _output_get (set `self.controleStamina` (- (`self.controleStamina`) 2)))
    (`KismetSystemLibrary.PrintString` (`KismetStringLibrary.Conv_IntToString` _output_get) true true (struct :`R` 1.0 :`B` 0.950709 :`A` 1.0))))

(event `self.ReceiveActorOnClicked`
  (params (ButtonPressed :type "Key Structure"))
  (`|ExecutionSequence`
    (:`then_0`
      (set `self.confere2seg` true))
    (:`then_1`
      (bind _output_get (set `self.controleStamina` (+ (`self.controleStamina`) 1)))
      (`KismetSystemLibrary.PrintString` (`KismetStringLibrary.Conv_IntToString` _output_get)))))

(fn `UserConstructionScript`)